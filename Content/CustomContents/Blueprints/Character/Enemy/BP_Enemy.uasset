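; Enemy character Blueprint for regular, boss and "Slave" enemies, handling combat, weapons and HUD.
; Detection overlap or damage targets the player, who feeds a per-tick motion warp target; damage also drives attack-system states, knockback, floating numbers, death and boss phase two.
; Timer-triggered sphere traces along sword or arm points damage the player.
; Fist, sword and gun switches update the Blackboard; eye emission color signals idle, battle or slave.
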(event `self.ReceiveTick`
  (params (DeltaSeconds :type "Float (single-precision)"))
  ; Tick
  (bind _targetcharacter (`self.TargetCharacter`)
    (:`then`
      (bind _motionwarping (`self.MotionWarping`)
        (:`then`
          (`MotionWarpingComponent.AddOrUpdateWarpTarget` _motionwarping (make `MotionWarpingTarget` "Warp" (+ (`self.K2_GetActorLocation` _targetcharacter) (* (`self.GetActorForwardVector` _targetcharacter) 200.0)) (`self.K2_GetActorRotation` _targetcharacter) null "None")))
        (:`else`)))
    (:`else`)))

(event `OnAimTarget`
  (params (Activate :type Boolean))
  ; OnAimTarget
  (`/Game/CustomContents/UI/WB/Combat/WB_HUD.SetDetailTargetVisible` (`self.WB_HUD`) Activate))

(event `OnEnemyDialog`
  (params (Dialog :type String))
  ; OnEnemyDialog
  (`/Game/CustomContents/UI/WB/Combat/WB_HUD.OnEnemyDialog` (`self.WB_HUD`) Dialog))

(event `SpawnSlave`
  (bind _mesh (`self.Mesh`))
  ;[0.15 0.07641 0.002757 0.5] SpawnSlave
  (`/Game/CustomContents/Components/BPC_StatSystem.InitSlave` (`self.BPC_StatSystem`))
  (`KismetArrayLibrary.Array_Add` (`self.Tags`) "Slave")
  (`self.SetTargetCharacter` (`GameplayStatics.GetPlayerController` 0))
  ; Slave Blue Eye
  (bind _returnvalue (`PrimitiveComponent.CreateDynamicMaterialInstance` _mesh 0 (`PrimitiveComponent.GetMaterial` _mesh 0) "None"))
  (`MaterialInstanceDynamic.SetVectorParameterValue` _returnvalue "Emission Color" (struct :`G` 0.821556 :`B` 1.0 :`A` 1.0))
  ; Slave On Battle!
  (`|ExecutionSequence`
    (:`then_0`
      (`PrimitiveComponent.SetCollisionEnabled` (`self.CapsuleComponent`) "QueryOnly")
      (`self.Boost`))
    (:`then_1`
      (set `self.Damage Causer` (`GameplayStatics.GetPlayerController` 0)))
    (:`then_2`
      (`self.SetBackEnemyLocation` (`self.Damage Causer`) 20.0) ; Hit시 DamageCauser방향으로 이동
      (`/Game/CustomContents/Components/BPC_EnemyAttackSystem.SetCurrentState` (`self.BPC_EnemyAttackSystem`) "NewEnumerator6"))))

(event `self.TempDetector.OnComponentBeginOverlap`
  (params (OverlappedComponent :type "PrimitiveComponent Object Reference") (OtherActor :type "Actor Object Reference") (OtherComp :type "PrimitiveComponent Object Reference") (OtherBodyIndex :type Integer) (bFromSweep :type Boolean) (SweepResult :type "HitResult Structure (by ref)"))
  ; OnBegin(TmpDector)
  (if (`self.IsPlayEnable`)
    (bind _asbp_player_character (cast `/Game/CustomContents/Blueprints/Character/Player/BP_PlayerCharacter` OtherActor))
    (set `self.TargetCharacter` _asbp_player_character)
    ;;[0.15 0.03048 0 0.5] ChangeState
    (`/Game/CustomContents/UI/BP/BP_UI.UpdateCombatState` (`/Game/CustomContents/UI/BP/BPC_UserInterface.BP UI` (`self.BPC_UserInterface`)) "NewEnumerator1")
    ; Player Die Check
    (if (not (`self.bPlayerDiedBinded`))
      (add `/Game/CustomContents/Blueprints/Character/Player/BP_PlayerCharacter.OnPlayerDied` (`self.TargetCharacter`) (delegate `ChangeToIdle`))
      (set `self.bPlayerDiedBinded` false))))

(event `self.ReceiveBeginPlay`
  (bind _bpc_enemyattacksystem (`self.BPC_EnemyAttackSystem`))
  (bind _mesh (`self.Mesh`))
  ; Init
  (`|ExecutionSequence`
    (:`then_0`
      ;; Comment
      (set `self.immortal` true)
      (`KismetSystemLibrary.Delay` 1.0)
      (set `self.immortal` false))
    (:`then_1`
      ;; InitMinimap
      (`PrimitiveComponent.SetVisibleInSceneCaptureOnly` (`self.SightPaperSprite`) true)
      (`PrimitiveComponent.SetVisibleInSceneCaptureOnly` (`self.EnemyIndicator Sprite`) true)
      (`PrimitiveComponent.SetHiddenInSceneCapture` (`self.Mesh`) true))
    (:`then_2`
      ;; InitDebugState
      (bind _debugenable (`/Game/CustomContents/UI/BP/BPC_UserInterface.DebugDraw` (`self.BPC_UserInterface`)))
      (bind _output_get (set `self.Debug Enable` _debugenable))
      (`SceneComponent.SetHiddenInGame` (`self.TempDetector`) (== _output_get 0) false))
    (:`then_3`
      ;; Begin-Set Animation BP
      (bind _asabp_enemy (cast `/Game/CustomContents/Blueprints/Character/Enemy/ABP_Enemy` (`SkeletalMeshComponent.GetAnimInstance` (`self.Mesh`))))
      (bind _output_get_2 (set `self.AnimationBP` _asabp_enemy))
      (set `/Game/CustomContents/Blueprints/Character/Enemy/ABP_Enemy.Enemy` self _output_get_2))
    (:`then_4`
      ;; Comment
      (`self.InitHUD`)
      ;; InitInstance
      (bind _aspunk_game_instance (cast `/Game/CustomContents/Blueprints/PunkGameInstance` (`GameplayStatics.GetGameInstance`)))
      (set `self.PunkGameInstance` _aspunk_game_instance))
    (:`then_5`
      ;; IsBossType
      (if (`/Game/CustomContents/Components/BPC_StatSystem.IsBossType` (`self.BPC_StatSystem`))
        (if (`self.IsPlayEnable`)
          (set `/Game/CustomContents/Components/BPC_EnemyAttackSystem.ViewDistance` 3000.0 _bpc_enemyattacksystem)
          (else
            (set `/Game/CustomContents/Components/BPC_EnemyAttackSystem.ViewDistance` 0.0 _bpc_enemyattacksystem)))))
    (:`then_6`
      ;; Set Green Eye
      (bind _returnvalue (`PrimitiveComponent.CreateDynamicMaterialInstance` _mesh 0 (`PrimitiveComponent.GetMaterial` _mesh 0) "None"))
      (`MaterialInstanceDynamic.SetVectorParameterValue` _returnvalue "Emission Color" (struct :`G` 1.0 :`A` 1.0)))))

(event `ChangeToIdle`
  ; Player Die Check
  (`/Game/CustomContents/Components/BPC_EnemyAttackSystem.SetCurrentState` (`self.BPC_EnemyAttackSystem`) "NewEnumerator0")
  (set `/Game/CustomContents/Components/BPC_EnemyAttackSystem.IsPlayerDead` true (`self.BPC_EnemyAttackSystem`)))

(event `OnDamage`
  (params (Damage :type "Float (double-precision)") (Critical :type Boolean) (`Instigated By` :type "Controller Object Reference") (`Damage Causer` :type "Actor Object Reference"))
  (if (not (`self.Is Dead`))
    (`|ExecutionSequence`
      (:`then_0`
        ; Tick Boss Phase
        (`/Game/CustomContents/Blueprints/PunkGameInstance.TickBossPhase` (`self.PunkGameInstance`)))
      (:`then_1`
        ; OnDamaged
        (set `self.Damage` Damage)
        (set `self.Critical` Critical)
        (`self.SetTargetCharacter` `Instigated By`)
        (set `self.IsHit` true)
        (set `self.Damage Causer` `Damage Causer`)
        (`self.Boost`)
        ; Immortal
        (if (not (`self.immortal`))
          ;[0.15 0.03048 0 0.5] ChangeState
          (`/Game/CustomContents/UI/BP/BP_UI.UpdateCombatState` (`/Game/CustomContents/UI/BP/BPC_UserInterface.BP UI` (`self.BPC_UserInterface`)) "NewEnumerator1")
          ; DecreaseHealth
          (`self.ShowFloatingNumber` (`self.Damage`) (`self.Critical`))
          (bind _isdead (`/Game/CustomContents/Components/BPC_StatSystem.DecreaseHealth` (`self.BPC_StatSystem`) (`self.Damage`) (`self.WB_HUD`)))
          (`self.UpdateBossHealth`)
          (`|ExecutionSequence`
            (:`then_0`
              (bind _output_get (set `self.Is Dead` _isdead))
              (if _output_get
                ;[0.15 0.03234 0.04202 0.5] OnDead
                (`/Game/CustomContents/Components/BPC_EnemyAttackSystem.SetCurrentState` (`self.BPC_EnemyAttackSystem`) "NewEnumerator4")
                (`|PlayMontage` (`self.Mesh`) "/Game/CustomContents/Animation/Montages/Death_Montage.Death_Montage"
                  (:`then`
                    ;;[0.15 0.02547 9.4e-05 0.5] 사망시 처리, 콜리전을 Off후,  5초후 액터 제거
                    (`PrimitiveComponent.SetCollisionEnabled` (`self.CapsuleComponent`) "NoCollision")
                    (`|ExecutionSequence`
                      (:`then_0`
                        ; IsBossType
                        (if (`/Game/CustomContents/Components/BPC_StatSystem.IsBossType` (`self.BPC_StatSystem`))
                          ; Player Win!!!
                          (`/Game/CustomContents/UI/WB/Combat/WB_UI.OnEnemySkillDialog` (`/Game/CustomContents/UI/BP/BPC_UserInterface.WB UI` (`self.BPC_UserInterface`)) (`/Game/CustomContents/Blueprints/PunkGameInstance.GetPlayerWinDialog` (`self.PunkGameInstance`)))
                          (`KismetSystemLibrary.Delay` 5.0)
                          ;[0.15 0.03048 0 0.5] GameOver
                          (`/Game/CustomContents/UI/BP/BP_UI.UpdateCombatState` (`/Game/CustomContents/UI/BP/BPC_UserInterface.BP UI` (`self.BPC_UserInterface`)) "NewEnumerator2")))
                      (:`then_1`
                        (`KismetSystemLibrary.Delay` 5.0)
                        (`self.K2_DestroyActor`)))))
                (else
                  ; OnHit
                  (`self.SetBackEnemyLocation` (`self.Damage Causer`) 20.0) ; Hit시 DamageCauser방향으로 이동
                  (`/Game/CustomContents/Components/BPC_EnemyAttackSystem.SetCurrentState` (`self.BPC_EnemyAttackSystem`) "NewEnumerator6")
                  ; HitEnd
                  (`KismetSystemLibrary.Delay` 1.5)
                  (set `self.IsHit` false)
                  (`/Game/CustomContents/Components/BPC_EnemyAttackSystem.SetCurrentState` (`self.BPC_EnemyAttackSystem`) "NewEnumerator0"))))
            (:`then_1`
              ; IsBossType
              (if (`/Game/CustomContents/Components/BPC_StatSystem.IsBossType` (`self.BPC_StatSystem`))
                ; CheckBossHealthPer
                (if (< (* (`/Game/CustomContents/Components/BPC_StatSystem.HealthPercent` (`self.BPC_StatSystem`)) 100.0) (`/Game/CustomContents/Blueprints/PunkGameInstance.GetConfigData` (`self.PunkGameInstance`) "Phase2BossHPPer"))
                  ; SetPhase2
                  (if (== (`/Game/CustomContents/Blueprints/PunkGameInstance.GetBossPhase` (`self.PunkGameInstance`)) 1)
                    (set `/Game/CustomContents/Blueprints/PunkGameInstance.BossPhase` 2 (`self.PunkGameInstance`))
                    ; Phase2 Warning
                    (`/Game/CustomContents/UI/WB/Combat/WB_UI.OnEnemySkillDialog` (`/Game/CustomContents/UI/BP/BPC_UserInterface.WB UI` (`self.BPC_UserInterface`)) (`/Game/CustomContents/Blueprints/PunkGameInstance.GetPhase2EnterDialog` (`self.PunkGameInstance`)))))))))))))

(event `self.ReceiveAnyDamage`
  (params (Damage :type "Float (single-precision)") (DamageType :type "DamageType Object Reference") (InstigatedBy :type "Controller Object Reference") (DamageCauser :type "Actor Object Reference"))
  ; OnDamaged
  (`KismetSystemLibrary.PrintString` "Deprecated Enemy ApplyDamage" false false))

(event `StartAttack`
  ; OnStartAttack
  (bind _returnvalue (`KismetSystemLibrary.K2_SetTimerDelegate` (delegate `Attack`) 0.01))
  (set `self.AttackTimerHandler` _returnvalue))

(event `StopAttack`
  ; OnStopAttack
  (`KismetSystemLibrary.K2_ClearAndInvalidateTimerHandle` (`self.AttackTimerHandler`)))

(event `Attack`
  ; OnAttack
  (`self.TraceToAttack` (`self.TraceStartLoc`) (`self.TraceEndLoc`)))

(event `OnBattleMode`
  (bind _mesh (`self.Mesh`))
  ; Enter BattleMode
  (bind _returnvalue (`PrimitiveComponent.CreateDynamicMaterialInstance` _mesh 0 (`PrimitiveComponent.GetMaterial` _mesh 0) "None"))
  (`MaterialInstanceDynamic.SetVectorParameterValue` _returnvalue "Emission Color" (struct :`R` 1.0 :`G` 0.017854 :`A` 1.0)))

(event `SetLeftSwordTraceLoc`
  ; SetLeftSwordTraceLocation
  (set `self.TraceStartLoc` (`self.GetTraceLocStart` (`self.LeftSwordRef`)))
  (set `self.TraceEndLoc` (`self.GetTraceLocEnd` (`self.LeftSwordRef`))))

(event `SetRightSwordTraceLoc`
  ; SetRightSwordTraceLocation
  (set `self.TraceStartLoc` (`self.GetTraceLocStart` (`self.RightSwordRef`)))
  (set `self.TraceEndLoc` (`self.GetTraceLocEnd` (`self.RightSwordRef`))))

(event `Boost`
  ; Boost
  (`|ExecutionSequence`
    (:`then_0`
      ;; Boost
      (set `/Game/CustomContents/Components/BPC_EnemyAttackSystem.ChaseSpeed` (* (`self.MoveSpeed`) 2.0) (`self.BPC_EnemyAttackSystem`)))
    (:`then_2`)
    (:`then_3`)))

(event `SetRightArmTraceLocation`
  ; SetRightArmTraceLocation [오른쪽 주먹을 Trace Location으로 설정]
  (set `self.TraceStartLoc` (`self.GetTraceLocStart` null))
  (set `self.TraceEndLoc` (`self.GetTraceLocEnd` null)))

(event `SwitchWeaponToFist`
  ;[0.0787 0.15 0.1014 0.5] 무기 전환
  ;; SwitchWeaponToFist
  (`self.SwitchToFist`))

(event `SwitchWeaponToSword`
  ;[0.0787 0.15 0.1014 0.5] 무기 전환
  ;; SwitchWeaponToSword
  (`self.SwitchToSwords`))

(event `SwitchWeaponToGun`
  ;[0.0787 0.15 0.1014 0.5] 무기 전환
  ;; SwitchWeaponToGun
  (`self.SwitchToGun`))

(fn `DetachWeapon`
  (params (Target :type "Actor Object Reference"))
  (`SceneComponent.K2_DetachFromComponent` (`Actor.RootComponent` Target) "KeepRelative" "KeepRelative" "KeepRelative" true))

(fn `GetHitAnimation`
  (params (Array :type "Array of AnimMontage Object Reference"))
  (returns (Animation :type "AnimMontage Object Reference"))
  (return (`|GetArrayItem` Array (`KismetMathLibrary.RandomIntegerInRange` 0 (- (`KismetArrayLibrary.Array_Length` Array) 1)))))

(fn `GetTraceLocEnd`
  (params (Ref :type "Actor Object Reference"))
  (returns (Location :type "Vector Structure"))
  (bind _asbp_sword (cast `/Game/CustomContents/Blueprints/Weapon/BP_Sword` Ref)
    (:`then`
      (return (`SceneComponent.K2_GetComponentLocation` (`/Game/CustomContents/Blueprints/Weapon/BP_Sword.TraceEnd` _asbp_sword))))
    (:`CastFailed`
      (return (`SceneComponent.K2_GetComponentLocation` (`self.RightArmEnd`))))))

(fn `GetTraceLocStart`
  (params (Target :type "/Game/CustomContents/Blueprints/Weapon/BP_Sword Object Reference"))
  (returns (Location :type "Vector Structure"))
  (bind _asbp_sword (cast `/Game/CustomContents/Blueprints/Weapon/BP_Sword` Target)
    (:`then`
      (return (`SceneComponent.K2_GetComponentLocation` (`/Game/CustomContents/Blueprints/Weapon/BP_Sword.TraceStart` _asbp_sword))))
    (:`CastFailed`
      (return (`SceneComponent.K2_GetComponentLocation` (`self.RightArmStart`))))))

(fn `InitHUD`
  (locals (IsBoss :type Boolean))
  (bind _bpc_statsystem (`self.BPC_StatSystem`))
  (bind _aswb_hud (cast `/Game/CustomContents/UI/WB/Combat/WB_HUD` (`WidgetComponent.GetUserWidgetObject` (`self.Widget`))))
  (set `self.WB_HUD` _aswb_hud)
  (bind _output_get (set `local.IsBoss` (`/Game/CustomContents/Components/BPC_StatSystem.IsBossType` (`self.BPC_StatSystem`))))
  (if _output_get
    ; InitEnemyUI
    (`/Game/CustomContents/UI/BP/BPC_UserInterface.UpdateBossHealth` (`self.BPC_UserInterface`) (`/Game/CustomContents/Components/BPC_StatSystem.CurrentHealth` _bpc_statsystem) (`/Game/CustomContents/Components/BPC_StatSystem.MaxHealth` _bpc_statsystem)))
  (`/Game/CustomContents/UI/WB/Combat/WB_HUD.SetDetailTargetVisible` (`self.WB_HUD`) (`local.IsBoss`)) ; 보스 일떄 보인다
  ; HealthBarDisaply
  (`/Game/CustomContents/UI/WB/Combat/WB_HUD.SetActivateHealthBar` (`self.WB_HUD`) (not (`local.IsBoss`))) ; 보스 아닐때 보인다
)

(fn `IsPlayEnable`
  (returns (Enable :type Boolean))
  (if (and (`KismetMathLibrary.BooleanNOR` (`self.Is Dead`)) (== (`/Game/CustomContents/Blueprints/PunkGameInstance.BossPhase` (`self.PunkGameInstance`)) 1))
    (return true)
    (else
      (return false))))

(fn `Play Hit Animation`
  (params (Array :type "Array of AnimMontage Object Reference"))
  (returns (DelayTime :type "Float (single-precision)"))
  (bind _returnvalue (`self.PlayAnimMontage` (`|GetArrayItem` Array (`KismetMathLibrary.RandomIntegerInRange` 0 (- (`KismetArrayLibrary.Array_Length` Array) 1)))))
  (return _returnvalue))

(fn `SetBackEnemyLocation`
  (params (`Damage Causer` :type "Actor Object Reference") (`Back Value` :type "Float (double-precision)"))
  (`self.K2_SetActorLocation` (+ (* (`self.GetActorForwardVector` `Damage Causer`) `Back Value`) (`self.K2_GetActorLocation`))))

(fn `SetTargetCharacter`
  (params (Instigator :type "Controller Object Reference"))
  (`/Engine/EditorBlueprintResources/StandardMacros.IsValid` Instigator
    (:`Is Valid`
      (bind _asbp_player_character (cast `/Game/CustomContents/Blueprints/Character/Player/BP_PlayerCharacter` (`Controller.K2_GetPawn` Instigator)))
      (set `self.TargetCharacter` _asbp_player_character)
      (`/Game/CustomContents/Components/BPC_EnemyAttackSystem.SetCurrentState` (`self.BPC_EnemyAttackSystem`) "NewEnumerator2"))))

(fn `ShowFloatingNumber`
  (params (DamageDone :type "Float (double-precision)") (Critical :type Boolean))
  (bind (_returnvalue_x _returnvalue_y _returnvalue_z) (`KismetMathLibrary.BreakVector` (`self.K2_GetActorLocation`)))
  (bind _returnvalue (`KismetMathLibrary.MakeVector` _returnvalue_x _returnvalue_y (+ _returnvalue_z 50.0)))
  (if Critical
    (bind _returnvalue_2 (`|CreateWidget` "/Game/CustomContents/UI/WB/Combat/WB_CriticalFloatingNumber.WB_CriticalFloatingNumber_C" null DamageDone _returnvalue))
    (`UserWidget.AddToViewport` _returnvalue_2 0)
    (else
      (bind _returnvalue_3 (`|CreateWidget` "/Game/CustomContents/UI/WB/Combat/WB_FloatingNumber.WB_FloatingNumber_C" null DamageDone _returnvalue))
      (`UserWidget.AddToViewport` _returnvalue_3 0))))

(fn `SpawnWeaponAndAttach`
  (params (Class :type "Actor Class Reference") (InputPin :type Name))
  (returns (ReturnValue :type "Actor Object Reference"))
  (bind _returnvalue (`|SpawnActorFromClass` Class (`KismetMathLibrary.MakeTransform` (0.0 0.0 0.0)) "Undefined" "MultiplyWithRoot" null null))
  (`self.K2_AttachToComponent` _returnvalue (`self.Mesh`) InputPin "KeepRelative" "KeepRelative" "KeepRelative" true)
  (return _returnvalue))

(fn `SwitchToFist`
  (switch `/Game/CustomContents/Blueprints/EEnemyWeaponType` (`self.CurrentWeapon`)
    (:`NewEnumerator0`
      (bind _output_get (set `self.CurrentWeapon` "NewEnumerator2"))
      (`BlackboardComponent.SetValueAsEnum` (`AIBlueprintHelperLibrary.GetBlackboard` null) (`self.CurrentWeaponName`) _output_get)
      (`self.DetachWeapon` (`self.LeftSwordRef`))
      (`self.DetachWeapon` (`self.RightSwordRef`)))
    (:`NewEnumerator1`
      (bind _output_get_2 (set `self.CurrentWeapon` "NewEnumerator2"))
      (`BlackboardComponent.SetValueAsEnum` (`AIBlueprintHelperLibrary.GetBlackboard` null) (`self.CurrentWeaponName`) _output_get_2)
      (`self.DetachWeapon` (`self.GunRef`)))))

(fn `SwitchToGun`
  (switch `/Game/CustomContents/Blueprints/EEnemyWeaponType` (`self.CurrentWeapon`)
    (:`NewEnumerator2`
      (bind _output_get (set `self.CurrentWeapon` "NewEnumerator1"))
      (`BlackboardComponent.SetValueAsEnum` (`AIBlueprintHelperLibrary.GetBlackboard` null) (`self.CurrentWeaponName`) _output_get)
      (`self.SpawnWeaponAndAttach` "/Game/CustomContents/Blueprints/Weapon/BP_Gun.BP_Gun_C" (`self.GunSocketName`)))
    (:`NewEnumerator0`
      (bind _output_get_2 (set `self.CurrentWeapon` "NewEnumerator1"))
      (`BlackboardComponent.SetValueAsEnum` (`AIBlueprintHelperLibrary.GetBlackboard` null) (`self.CurrentWeaponName`) _output_get_2)
      (`self.DetachWeapon` (`self.LeftSwordRef`))
      (`self.DetachWeapon` (`self.RightSwordRef`))
      (`self.GunRef` ; Gun이 이미 존재하면 스폰하지 않고 Attach,\n없으면 스폰 후 Attach
        (:`then`
          (`self.K2_AttachToComponent` (`self.GunRef`) (`self.Mesh`) (`self.GunSocketName`) "KeepRelative" "KeepRelative" "KeepRelative" true))
        (:`else`
          (`self.SpawnWeaponAndAttach` "/Game/CustomContents/Blueprints/Weapon/BP_Gun.BP_Gun_C" (`self.GunSocketName`)))))))

(fn `SwitchToSwords`
  (switch `/Game/CustomContents/Blueprints/EEnemyWeaponType` (`self.CurrentWeapon`)
    (:`NewEnumerator2`
      (bind _output_get (set `self.CurrentWeapon` "NewEnumerator0"))
      (`BlackboardComponent.SetValueAsEnum` (`AIBlueprintHelperLibrary.GetBlackboard` null) (`self.CurrentWeaponName`) _output_get)
      (`self.LeftSwordRef` ; Left Sword가 이미 존재하면 스폰하지 않고 Attach,\n없으면 스폰 후 Attach
        (:`then`
          (`self.K2_AttachToComponent` (`self.LeftSwordRef`) (`self.Mesh`) (`self.LeftWeaponSocketName`) "KeepRelative" "KeepRelative" "KeepRelative" true)
          (`self.K2_AttachToComponent` (`self.RightSwordRef`) (`self.Mesh`) (`self.RightWeaponSocketName`) "KeepRelative" "KeepRelative" "KeepRelative" true))
        (:`else`
          (`self.SpawnWeaponAndAttach` "/Game/CustomContents/Blueprints/Weapon/BP_Sword.BP_Sword_C" (`self.LeftWeaponSocketName`))
          (`self.SpawnWeaponAndAttach` "/Game/CustomContents/Blueprints/Weapon/BP_Sword.BP_Sword_C" (`self.RightWeaponSocketName`)))))
    (:`NewEnumerator1`
      (bind _output_get_2 (set `self.CurrentWeapon` "NewEnumerator0"))
      (`BlackboardComponent.SetValueAsEnum` (`AIBlueprintHelperLibrary.GetBlackboard` null) (`self.CurrentWeaponName`) _output_get_2)
      (`self.DetachWeapon` (`self.GunRef`))
      (`self.LeftSwordRef` ; Left Sword가 이미 존재하면 스폰하지 않고 Attach,\n없으면 스폰 후 Attach
        (:`then`
          (`self.K2_AttachToComponent` (`self.LeftSwordRef`) (`self.Mesh`) (`self.LeftWeaponSocketName`) "KeepRelative" "KeepRelative" "KeepRelative" true)
          (`self.K2_AttachToComponent` (`self.RightSwordRef`) (`self.Mesh`) (`self.RightWeaponSocketName`) "KeepRelative" "KeepRelative" "KeepRelative" true))
        (:`else`
          (`self.SpawnWeaponAndAttach` "/Game/CustomContents/Blueprints/Weapon/BP_Sword.BP_Sword_C" (`self.LeftWeaponSocketName`))
          (`self.SpawnWeaponAndAttach` "/Game/CustomContents/Blueprints/Weapon/BP_Sword.BP_Sword_C" (`self.RightWeaponSocketName`)))))))

(fn `TraceToAttack`
  (params (TraceStartLocation :type "Vector Structure") (TraceEndLocation :type "Vector Structure"))
  (locals (NewLocalVar :type "Array of EObjectTypeQuery Enum"))
  (bind (_outhit _returnvalue) (`KismetSystemLibrary.SphereTraceSingleForObjects` TraceStartLocation TraceEndLocation (`self.AttackTraceRadius`) (`local.NewLocalVar`)))
  (if _returnvalue
    (bind _asbp_player_character (cast `/Game/CustomContents/Blueprints/Character/Player/BP_PlayerCharacter` (`.HitActor` (`GameplayStatics.BreakHitResult` _outhit))))
    (bind (_damage _critical) (`/Game/CustomContents/Components/BPC_StatSystem.GetDamage` (`self.BPC_StatSystem`)))
    (`/Game/CustomContents/Blueprints/Character/Player/BP_PlayerCharacter.OnDamage` _asbp_player_character _damage _critical (`self.GetController` self) self)))

(fn `UpdateBossHealth`
  (bind _bpc_statsystem (`self.BPC_StatSystem`))
  (if (`/Game/CustomContents/Components/BPC_StatSystem.IsBossType` (`self.BPC_StatSystem`))
    (`/Game/CustomContents/UI/BP/BPC_UserInterface.UpdateBossHealth` (`self.BPC_UserInterface`) (`/Game/CustomContents/Components/BPC_StatSystem.CurrentHealth` _bpc_statsystem) (`/Game/CustomContents/Components/BPC_StatSystem.MaxHealth` _bpc_statsystem)))
  (return))

(fn `UserConstructionScript`)