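; BP_SlaveSpawn is a spawner that adds slave enemies near the boss during its second phase.
; On BeginPlay it finds the boss-type BP_Enemy and the UI, and reads spawn delay and max count from PunkGameInstance config.
; A looping timer checks phase, live "Slave"-tagged count, cooldown timestamp and UI combat state.
; When all pass, a second timer spawns two slaves one second apart, then clears itself.
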(event `self.ReceiveBeginPlay`
  (`|ExecutionSequence`
    (:`then_0`
      ; Init
      (bind _aspunk_game_instance (cast `/Game/CustomContents/Blueprints/PunkGameInstance` (`GameplayStatics.GetGameInstance`)))
      (set `self.Punk Game Instance` _aspunk_game_instance)
      ; Get Boss Enemy
      (bind _outactors (`GameplayStatics.GetAllActorsOfClass` "/Game/CustomContents/Blueprints/Character/Enemy/BP_Enemy.BP_Enemy_C"))
      (for _array_element _outactors
        (if (`/Game/CustomContents/Components/BPC_StatSystem.IsBossType` (`/Game/CustomContents/Blueprints/Character/Enemy/BP_Enemy.BPC_StatSystem` _array_element))
          (set `self.BP_Boss` _array_element))))
    (:`then_1`
      ; Comment
      (bind _returnvalue (`GameplayStatics.GetActorOfClass` "/Game/CustomContents/UI/BP/BP_UI.BP_UI_C"))
      (set `self.BP_UI` _returnvalue))
    (:`then_2`
      ; Create Tick
      (bind _returnvalue_2 (`KismetSystemLibrary.K2_SetTimer` null "CheckSpawn" 1.0 true))
      (set `self.CheckSpawnTimer` _returnvalue_2))
    (:`then_3`
      ; Set Spawn Delay
      (set `self.SpawnDelay` (`KismetMathLibrary.FTrunc` (`/Game/CustomContents/Blueprints/PunkGameInstance.GetConfigData` (`self.Punk Game Instance`) "SpawnDelay"))))
    (:`then_4`
      ; Set Max Spawn
      (set `self.MaxSpawn` (`KismetMathLibrary.FTrunc` (`/Game/CustomContents/Blueprints/PunkGameInstance.GetConfigData` (`self.Punk Game Instance`) "MaxSpawnCount"))))))

(event `SpawnSlave`
  (bind (_returnvalue_x _returnvalue_y) (`KismetMathLibrary.BreakVector` (+ (`self.K2_GetActorLocation` (`self.BP_Boss`)) (* (`self.GetActorForwardVector` (`self.BP_Boss`)) (-50.0 0.0 0.0)))))
  ; Spawn Slave
  (bind _returnvalue (`|SpawnActorFromClass` "/Game/CustomContents/Blueprints/Character/Enemy/BP_Enemy.BP_Enemy_C" (`KismetMathLibrary.MakeTransform` (`KismetMathLibrary.MakeVector` _returnvalue_x _returnvalue_y 107.5)) "AdjustIfPossibleButAlwaysSpawn" "MultiplyWithRoot" null null))
  (`/Engine/EditorBlueprintResources/StandardMacros.IsValid` _returnvalue
    (:`Is Valid`
      (`/Game/CustomContents/Blueprints/Character/Enemy/BP_Enemy.SpawnSlave` _returnvalue)
      (set `self.SpawnCount` (- (`self.SpawnCount`) 1))
      (if (<= (`self.SpawnCount`) 0)
        (`KismetSystemLibrary.K2_ClearAndInvalidateTimerHandle` (`self.SpawnSlaveTimer`))))))

(event `CheckSpawn`
  ; Check Phase
  (if (== (`/Game/CustomContents/Blueprints/PunkGameInstance.GetBossPhase` (`self.Punk Game Instance`)) 2)
    ; Check Max Spawn Count
    (bind _outactors (`GameplayStatics.GetAllActorsOfClassWithTag` "/Game/CustomContents/Blueprints/Character/Enemy/BP_Enemy.BP_Enemy_C" "Slave"))
    (if (<= (`KismetArrayLibrary.Array_Length` _outactors) (`self.MaxSpawn`))
      ; Check Next Spawn Time
      (if (> (`/Game/CustomContents/UI/BP/BPFL_Time.GetTimestamp`) (`self.NextSpawnTime`))
        ; IsCombatState
        (if (`|EnumEquality` (`/Game/CustomContents/UI/BP/BP_UI.CombatState` (`self.BP_UI`)) "NewEnumerator1")
          ; Set Next SpawnTime
          (set `self.NextSpawnTime` (+ (`/Game/CustomContents/UI/BP/BPFL_Time.GetTimestamp`) (`self.SpawnDelay`)))
          (bind _returnvalue (`KismetSystemLibrary.K2_SetTimerDelegate` (delegate `SpawnSlave`) 1.0 true))
          (set `self.SpawnCount` 2)
          (set `self.SpawnSlaveTimer` _returnvalue))))))

(fn `UserConstructionScript`)